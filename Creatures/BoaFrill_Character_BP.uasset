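; BoaFrill creature Blueprint that is tamed by eating dropped dino eggs, crediting affinity to the team of the player who dropped them.
; While untargeted and past an affinity cooldown, its server timer octree-searches for eggs, then a looping timer pauses the AI brain and walks it over.
; Affinity scales from the egg species' required tame affinity and the game's taming multiplier, taming the creature once full.
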(event Custom|MoveToEgg
  (bind _eggreference (Variables|Local/DoNotEdit|GetEggReference))
  ;[1 0.7458 0.2266] AI brain behavior
  (if (Utilities|IsValid _eggreference)
    (bind _asprimaldinoaicontroller (Utilities|Casting|CastToPrimalDinoAIController (Pawn|GetController)))
    (AI|Navigation|MovetoLocation _asprimaldinoaicontroller (Transformation|GetActorLocation _eggreference) -1.0 true true false true 0 false)))

(event Custom|StartEggMoving
  ;[1 0.7458 0.2266] AI brain behavior
  (Utilities|IsValid (Variables|Default|GetTarget)
    (:Is%20Valid
      (CallFunction|RestartBrain))
    (:Is%20Not%20Valid
      (Utilities|FlowControl|DoOnce false
        (:Completed
          (Utilities|FlowControl|Sequence
            (:then_0
              (bind _asprimaldinoaicontroller (Utilities|Casting|CastToPrimalDinoAIController (Pawn|GetController)))
              (Class|PrimalDinoAIController|PauseBrainComponent _asprimaldinoaicontroller "ATTRACTED")
              (CallFunction|MovetoEgg)
              (Utilities|Time|SetTimerbyFunctionName self "RestartBrain" 1e+01)
              (if (Variables|Default|GetShouldPlayEggFoundStartle)
                (if (not (Variables|Local/DoNotEdit|GetPlayedFoundEggAnim))
                  (Class|PrimalCharacter|PlayAnimEx (Variables|Default|GetStartledAnimationRightDefault) 1.0 "None" true true false false false 0.0 0.0)
                  (Variables|Local/DoNotEdit|SetPlayedFoundEggAnim true))))
            (:then_1
              (Utilities|FlowControl|DoOnce false) ; enters at Reset
            )))))))

(event Custom|DissolveEggItem
  (bind _eggreference (Variables|Local/DoNotEdit|GetEggReference))
  ;[1 0 0.0858] Dissolve egg (visual and destroying world object)
  (bind _alpha (Timeline|Timeline_0 PlayFromStart)
    (:Update
      (if (not (Networking|IsDedicatedServer))
        (Utilities|IsValid (Variables|Local/DoNotEdit|GetEggReference)
          (:Is%20Valid
            (bind _asmaterialinstancedynamic (Utilities|Casting|CastToMaterialInstanceDynamic (Utilities|Array|Get(acopy) (Variables|/Script/Engine.MeshComponent|GetMaterials (Variables|Character|GetMesh)))))
            (Rendering|Material|SetScalarParameterValue _asmaterialinstancedynamic "DissolvePercent" _alpha :!class /Script/Engine.MaterialInstanceDynamic)))))
    (:Finished
      (Utilities|IsValid _eggreference
        (:Is%20Valid
          (Effects|SpawnEmitteratLocation 0 (Transformation|GetActorLocation _eggreference) "0, 0, 0" true false)
          (Actor|DestroyActor _eggreference))))))

(event Custom|EatEgg
  (bind _eggreference (Variables|Local/DoNotEdit|GetEggReference))
  (bind _eggreference_2 (Variables|Local/DoNotEdit|GetEggReference))
  (bind _droppedbyactor (Variables|/Script/ShooterGame.DroppedItem|GetDroppedByActor _eggreference))
  ;[0.6604 0.187 1] Eat egg (adds taming)
  (bind _returnvalue (Class|VictoryCore|GetClassDefaultObject (Variables|/Script/ShooterGame.PrimalItem|GetEggDinoClassToSpawn (Variables|/Script/ShooterGame.DroppedItem|GetMyItem _eggreference))))
  (bind _asprimaldinocharacter (Utilities|Casting|CastToPrimalDinoCharacter _returnvalue))
  (Utilities|IsValid _droppedbyactor
    (:Is%20Valid
      (bind _asshootercharacter (Utilities|Casting|CastToShooterCharacter _droppedbyactor))
      (CallFunction|IncreaseTamingAffinity _asshootercharacter (Variables|/Script/ShooterGame.PrimalDinoCharacter|GetRequiredTameAffinity _asprimaldinocharacter))
      (Class|PrimalCharacter|PlayAnimEx (Variables|Default|GetWakingConsumeFoodAnim) 1.0 "None" true true false false false 0.0 0.0)
      (Class|DroppedItemEgg|NetSpawnDinoEmitter _eggreference_2)
      (Actor|DestroyActor _eggreference_2)
      (CallFunction|ResetEggSeeking)
      (CallFunction|TameifAllowed))))

(event Custom|UpdateSeekEgg
  (bind _eggreference (Variables|Local/DoNotEdit|GetEggReference))
  ;[0.144 0.4663 1] UpdateSeekEgg
  (Utilities|IsValid _eggreference
    (:Is%20Valid
      (if (>= (Math|Vector|VectorLength (- (Transformation|GetActorLocation) (Transformation|GetActorLocation _eggreference))) 4e+02)
        (if (Class|Actor|BPIsA (Pawn|GetController) "/Script/ShooterGame.PrimalDinoAIController")
          (CallFunction|StartEggMoving))
        (else
          (CallFunction|EatEgg))))))

(event Custom|RestartBrain
  ;[1 0.7458 0.2266] AI brain behavior
  (Utilities|FlowControl|DoOnce false
    (:Completed
      (Utilities|FlowControl|Sequence
        (:then_0
          (bind _asprimaldinoaicontroller (Utilities|Casting|CastToPrimalDinoAIController (Pawn|GetController)))
          (Class|PrimalDinoAIController|ResumeBrainComponent _asprimaldinoaicontroller "NO LONGER ATTRACTED"))
        (:then_1
          (Utilities|FlowControl|DoOnce false) ; enters at Reset
        )))))

(event Custom|StartUpdateEggSeekTimer
  ;[0.6054 0.2299 1] Ensure seeking if we have valid egg target
  (if (not (Class|KismetSystemLibrary|IsTimerActive self "UpdateSeekEgg"))
    (Utilities|Time|SetTimerbyFunctionName self "UpdateSeekEgg" 0.5 true)))

(event EventBPTimerServer
  ;[0.2136 1 0.4575] Server Timer
  (|CallParentFunction)
  (if (Variables|Default|GetbCanBeTamed)
    (bind _returnvalue (Class|VictoryCore|StaticGetTimeSince (Class|Actor|GetWorld) (Variables|Local/DoNotEdit|GetLastTimeRecievedAffinity)))
    (if (>= _returnvalue (Variables|Default|GetEggCheckAfterAffinityCooldown))
      (Utilities|FlowControl|Sequence
        (:then_0
          ;[0.01142 1 0.8755] Don't hunt eggs with a target
          (if (not (Utilities|IsValid (Variables|Default|GetTarget)))
            ;[0.2816 0.5356 1] Find eggs nearby
            (if (Utilities|IsValid (Variables|Local/DoNotEdit|GetEggReference))
              (CallFunction|StartUpdateEggSeekTimer)
              (else
                (Variables|Local/DoNotEdit|SetPlayedFoundEggAnim false)
                (bind _returnvalue_2 (Class|VictoryCore|ServerOctreeOverlapActorsClass (Class|Actor|GetWorld) (Transformation|GetActorLocation) (Variables|Default|GetEggCheckRadius) "SPATIALNETWORKEDACTORS" (Variables|Default|GetEggFilterClass) false))
                (bind _array_element (Utilities|Array|ForEachLoopwithBreak _returnvalue_2 :!label _label)
                  (:LoopBody
                    (bind _asdroppeditemegg (Utilities|Casting|CastToDroppedItemEgg _array_element))
                    (if (Utilities|ClassIsChildOf (Variables|/Script/ShooterGame.PrimalItem|GetEggDinoClassToSpawn (Variables|/Script/ShooterGame.DroppedItem|GetMyItem _asdroppeditemegg)) "/Script/ShooterGame.PrimalDinoCharacter")
                      (Variables|Local/DoNotEdit|SetEggReference _asdroppeditemegg true)
                      (CallFunction|UpdateSeekEgg)
                      (CallFunction|StartUpdateEggSeekTimer)
                      (goto _label Break)))
                  (:Completed
                    (if (Utilities|IsValid (Variables|Default|GetTarget))
                      (CallFunction|ResetEggSeeking))))))
            (else
              (CallFunction|ResetEggSeeking))))
        (:then_1
          ;[1 0.8324 0.2217] Clear taming after affinity decrease
          (if (<= (Variables|Default|GetCurrentTameAffinity) 0.0)
            (Variables|Default|SetTamingTeamID 0 false)
            (if (not (Class|PrimalDinoCharacter|BPIsTamed))
              (Class|PrimalDinoCharacter|NetUpdateDinoNameStrings))))))
    (else
      (Variables|Default|SetbUseBPTimerServer false))))

(fn ConstructionScript
  (|CallParentFunction))

(fn BPSetupTamed
  (params (bWasJustTamed :type Boolean))
  (if (Variables|Default|GetbUseBPTimerServer)
    (Variables|Default|SetbUseBPTimerServer false)))

(fn UpdateTaming
  (params (ValueForTaming :type Float%20%28single-precision%29) (DroppedByShooterChar :type Primal%20Character%20Object%20Reference))
  (bind _returnvalue (Class|PrimalDinoCharacter|BPIsTamed))
  (LocalVariables|SetLocalTameAmount (+ (* ValueForTaming (Variables|Default|GetEggDinoAffinityInputMin)) (Variables|Default|GetEggTamingAffinityReturnedMin)))
  (if (<= (Variables|Default|GetCurrentTameAffinity) 0.0)
    (Variables|Default|SetTamingTeamID 0 false)
    (if _returnvalue
      _
      (else
        (Class|PrimalDinoCharacter|NetUpdateDinoNameStrings))))
  (if (not _returnvalue)
    (Class|PrimalCharacterStatusComponent|ModifyCurrentStatusValue (Variables|Default|GetMyCharacterStatusComponent) "Food" (Variables|Default|GetFoodToGetPerEggWhileTaming) false false false false 0 false false)
    (Utilities|FlowControl|Sequence
      (:then_0
        (bind _asprimaldinocharacter (Utilities|Casting|CastToPrimalDinoCharacter DroppedByShooterChar))
        (if (!= (Variables|/Script/ShooterGame.PrimalDinoCharacter|GetTamedAggressionLevel _asprimaldinocharacter) 0)
          (if (== 0 (Variables|Default|GetTamingTeamID))
            ;[1 1 1] Add affinity, update name stings, update waking tame
            (bind _asprimaldinocharacter_2 (Utilities|Casting|CastToPrimalDinoCharacter DroppedByShooterChar))
            (Variables|Default|SetTamingTeamID (Variables|/Script/Engine.Actor|GetTargetingTeam _asprimaldinocharacter_2) false)
            (Variables|Default|SetCurrentTameAffinity (+ (Variables|Default|GetCurrentTameAffinity) (LocalVariables|GetLocalTameAmount)) false)
            (Class|PrimalDinoCharacter|NetUpdateDinoNameStrings (Utilities|String|SelectString (Variables|/Script/ShooterGame.PrimalCharacter|GetTribeName _asprimaldinocharacter_2) (Variables|/Script/ShooterGame.PrimalDinoCharacter|GetTamerString _asprimaldinocharacter_2) (> (Utilities|String|Len (Variables|/Script/ShooterGame.PrimalCharacter|GetTribeName _asprimaldinocharacter_2)) 0)))
            (Variables|Local/DoNotEdit|SetLastTimeRecievedAffinity (Utilities|Time|GetGameTimeinSeconds))
            (if (not (Variables|Default|GetbIsWakingTame))
              (Variables|Default|SetbIsWakingTame true false))
            (else
              (bind _asprimaldinocharacter_3 (Utilities|Casting|CastToPrimalDinoCharacter DroppedByShooterChar))
              (if (== (Variables|/Script/Engine.Actor|GetTargetingTeam _asprimaldinocharacter_3) (Variables|Default|GetTamingTeamID))
                (Variables|Default|SetCurrentTameAffinity (+ (Variables|Default|GetCurrentTameAffinity) (LocalVariables|GetLocalTameAmount)) false)
                (Variables|Local/DoNotEdit|SetLastTimeRecievedAffinity (Utilities|Time|GetGameTimeinSeconds))
                (if (not (Variables|Default|GetbIsWakingTame))
                  (Variables|Default|SetbIsWakingTame true false)))))))
      (:then_1
        ;[1 1 1] If taming full, tame
        (CallFunction|TameifAllowed)))))

(fn IncreaseTamingAffinity
  (params (TamingPlayer :type Shooter%20Character%20Object%20Reference) (ValueForTaming :type Float%20%28single-precision%29))
  (bind _returnvalue (CallFunction|GetScaledAffinityBasedonDino ValueForTaming))
  (Utilities|FlowControl|Sequence
    (:then_0
      (if (== 0 (Variables|Default|GetTamingTeamID))
        (bind _asshootercharacter (Utilities|Casting|CastToShooterCharacter TamingPlayer)
          (:then
            (Variables|Default|SetTamingTeamID (Variables|/Script/Engine.Actor|GetTargetingTeam _asshootercharacter) false)
            (bind _asshootergamemode (Utilities|Casting|CastToShooterGameMode (Game|GetGameMode)))
            (Variables|Default|SetCurrentTameAffinity (+ (Variables|Default|GetCurrentTameAffinity) (* (Variables|/Script/ShooterGame.ShooterGameMode|GetTamingSpeedMultiplier _asshootergamemode) _returnvalue)) false)
            (Class|PrimalDinoCharacter|NetUpdateDinoNameStrings (Variables|/Script/ShooterGame.PrimalCharacter|GetTribeName _asshootercharacter))
            (Variables|Local/DoNotEdit|SetLastTimeRecievedAffinity (Utilities|Time|GetGameTimeinSeconds))
            (if (not (Variables|Default|GetbIsWakingTame))
              (Variables|Default|SetbIsWakingTame true false)
              (Variables|Default|SetTameIneffectivenessModifier (+ (/ (Variables|Default|GetTameIneffectivenessByAffinity) _returnvalue) (Variables|Default|GetTameIneffectivenessModifier)) false :!label _label)
              (Class|PrimalCharacterStatusComponent|ModifyCurrentStatusValue (Variables|Default|GetMyCharacterStatusComponent) "Food" (Variables|Default|GetFoodToGetPerEggWhileTaming) false false false false 0 false false)))
          (:CastFailed
            (goto _label)))
        (else
          (bind _asshootercharacter_2 (Utilities|Casting|CastToShooterCharacter TamingPlayer)
            (:then
              (if (== (Variables|/Script/Engine.Actor|GetTargetingTeam _asshootercharacter_2) (Variables|Default|GetTamingTeamID))
                (bind _asshootergamemode_2 (Utilities|Casting|CastToShooterGameMode (Game|GetGameMode)))
                (Variables|Default|SetCurrentTameAffinity (+ (Variables|Default|GetCurrentTameAffinity) (* _returnvalue (Variables|/Script/ShooterGame.ShooterGameMode|GetTamingSpeedMultiplier _asshootergamemode_2))) false)
                (Variables|Local/DoNotEdit|SetLastTimeRecievedAffinity (Utilities|Time|GetGameTimeinSeconds))
                (if (not (Variables|Default|GetbIsWakingTame))
                  (Variables|Default|SetbIsWakingTame true false)
                  (goto _label))))
            (:CastFailed
              (goto _label))))))
    (:then_1
      (return))))

(fn ResetEggSeeking
  (bind _self self)
  (Utilities|FlowControl|Sequence
    (:then_0
      (if (Class|KismetSystemLibrary|IsTimerActive _self "UpdateSeekEgg")
        (Utilities|Time|ClearTimerbyFunctionName _self "UpdateSeekEgg")))
    (:then_1
      (CallFunction|RestartBrain))
    (:then_2
      (return))))

(fn TameifAllowed
  (Utilities|FlowControl|Sequence
    (:then_0
      (if (>= (Variables|Default|GetCurrentTameAffinity) (Variables|Default|GetRequiredTameAffinity))
        (bind _asshootergamemode (Utilities|Casting|CastToShooterGameMode (Game|GetGameMode)))
        (bind _returnvalue (Class|ShooterGameMode|AllowTaming _asshootergamemode (Variables|Default|GetTamingTeamID)))
        (if _returnvalue
          (Class|PrimalDinoCharacter|TameDino 0 false 0 false false false)
          (Class|PrimalCharacter|PlayAnimEx "/Game/PrimalEarth/Dinos/Troodon/Animations/Troodon-Spot_Montage.Troodon-Spot_Montage" 1.0 "None" true false false false false 0.0 0.0))))
    (:then_1
      (return))))

(fn BPAdjustDamage
  (params (IncomingDamage :type Float%20%28single-precision%29) (TheDamageEvent :type Damage%20Event%20Structure) (EventInstigator :type Controller%20Object%20Reference) (DamageCauser :type Actor%20Object%20Reference) (bIsPointDamage :type Boolean) (PointHitInfo :type Hit%20Result%20Structure))
  (Utilities|FlowControl|Sequence
    (:then_0
      (if (Utilities|IsValid (Variables|Default|GetTarget))
        (CallFunction|ResetEggSeeking)))
    (:then_1
      (return IncomingDamage))))

(fn GetScaledAffinityBasedonDino
  (params (InputAffinity :type Float%20%28single-precision%29))
  (bind _eggtamingaffinityreturnedmin (Variables|Default|GetEggTamingAffinityReturnedMin))
  (bind _eggtamingaffinityreturnedmax (Variables|Default|GetEggTamingAffinityReturnedMax))
  (return (Math|Float|Clamp(Float) (Math|Float|Lerp _eggtamingaffinityreturnedmin _eggtamingaffinityreturnedmax (/ (- InputAffinity (Variables|Default|GetEggDinoAffinityInputMin)) (- (Variables|Default|GetEggDinoAffinityInputMax) (Variables|Default|GetEggDinoAffinityInputMin)))) _eggtamingaffinityreturnedmin _eggtamingaffinityreturnedmax)))