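; Eel creature Blueprint with shock attacks that go on a replicated cooldown, shown on clients through a particle effect and emissive glow.
; Attacks 2 and 3 start the cooldown and, with a gang, briefly draw chain beams to up to two nearby eels.
; A non-dedicated timer updates beam endpoints from a sphere overlap.
; Attack 3 rejects buff-immune characters and those whose drag weight exceeds a gang-scaled limit.
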(event Custom|AnimNotify_ShockAOEParticle
  (Components|Activation|Activate (Variables|Default|GetShockAOE) false)
  (Utilities|FlowControl|Delay 2.0)
  (Components|Activation|Deactivate (Variables|Default|GetShockAOE)))

(event Custom|StartParticles
  (if (not (Networking|IsDedicatedServer))
    (Components|Activation|Activate (Variables|Default|GetChainBeam1) false)
    (Variables|Default|SetbUseBPTimerNonDedicated true)
    (CallFunction|CheckNearbyandUpdateBeams)))

(event Custom|SetCanLightningAttackAfterDelay
  (bind _attackinfos (Variables|Default|GetAttackInfos))
  (Utilities|FlowControl|Delay (Math|Float|SelectFloat (.AttackInterval (Utilities|Struct|BreakDinoAttackInfo (Utilities|Array|Get(acopy) _attackinfos 3))) (.AttackInterval (Utilities|Struct|BreakDinoAttackInfo (Utilities|Array|Get(acopy) _attackinfos 2))) (Class|PrimalDinoCharacter|BPIsTamed)))
  (Variables|Default|SetCanLightningAttack true false))

(event Custom|UnsetFX
  (params (DiedCharacter :type Primal%20Character%20Object%20Reference))
  (Components|Activation|Deactivate (Variables|Default|GetCanLightningAttackEffect))
  (bind _asmaterialinstancedynamic (Utilities|Casting|CastToMaterialInstanceDynamic (Rendering|Material|GetMaterial (Variables|Character|GetMesh) 0)))
  (bind _returnvalue (Rendering|Material|GetVectorParameterValue _asmaterialinstancedynamic "Emissive - Color and Intensity" :!class /Script/Engine.MaterialInstanceDynamic))
  (Rendering|Material|SetVectorParameterValue _asmaterialinstancedynamic "Emissive - Color and Intensity" (Utilities|Struct|MakeLinearColor (.R (Utilities|Struct|BreakLinearColor _returnvalue)) (.G (Utilities|Struct|BreakLinearColor _returnvalue)) (.B (Utilities|Struct|BreakLinearColor _returnvalue)) (Variables|Default|GetminEmissive)) :!class /Script/Engine.MaterialInstanceDynamic))

(event Custom|ClearParticles
  (params (DelayTime :type Float%20%28single-precision%29))
  (if (not (Networking|IsDedicatedServer))
    (Utilities|FlowControl|Delay DelayTime)
    (Components|Activation|Deactivate (Variables|Default|GetChainBeam1))
    (Variables|Default|SetbUseBPTimerNonDedicated false)))

(event EventBeginPlay
  (Variables|Default|SetCanLightningAttack true false)
  (EventDispatchers|BindEventtoOnDied (delegate Custom|UnsetFX)))

(fn ConstructionScript
  (|CallParentFunction))

(fn BPDoAttack
  (params (AttackIndex :type Integer))
  (|CallParentFunction AttackIndex)
  (switch int AttackIndex
    (:2
      (if (> (Variables|Default|GetGangCount) 0)
        (CallFunction|StartParticles)
        (CallFunction|ClearParticles (Variables|Default|GetChainLifetime))))
    (:3
      (if (> (Variables|Default|GetGangCount) 0)
        (CallFunction|StartParticles)
        (CallFunction|ClearParticles (Variables|Default|GetChainLifetime)))))
  (Variables|Default|SetCanLightningAttack false false)
  (CallFunction|SetCanLightningAttackAfterDelay))

(fn BPTimerNonDedicated
  (CallFunction|CheckNearbyandUpdateBeams))

(fn UpdateChainBeamEnds
  (params (NearbyTeamEels :type Array%20of%20Actor%20Object%20References))
  ;[1 0.8754 0.3123] Early Out/Kill Particles if we don't have enough nearby eels
  (switch int (Utilities|Array|Length NearbyTeamEels)
    (:Default
      ;[0.4767 0.7726 1] Update all the beams we have enough eels for
      (bind (_array_element _array_index) (Utilities|Array|ForEachLoopwithBreak NearbyTeamEels :!label _label)
        (:LoopBody
          (if (< _array_index 2)
            (bind _asparticlesystemcomponent (Utilities|Casting|CastToParticleSystemComponent (Utilities|SelectObject (Variables|Default|GetChainBeam2) (Variables|Default|GetChainBeam1) (Math|Conversions|ToBoolean(Integer) _array_index))))
            (if (and (!= (Transformation|GetActorLocation _array_element) "0, 0, 0") (< (Math|Vector|VectorLength (- (Transformation|GetActorLocation _array_element) (Transformation|GetActorLocation))) (Variables|Default|GetGangOverlapRange)))
              (if (Variables|/Script/Engine.ParticleSystemComponent|GetbWasDeactivated _asparticlesystemcomponent)
                (Components|Activation|Activate _asparticlesystemcomponent false))
              (Effects|Components|ParticleSystem|SetVectorParameter _asparticlesystemcomponent "EndPoint" (Transformation|GetActorLocation _array_element))
              (else
                (Components|Activation|Deactivate _asparticlesystemcomponent)))
            (else
              (goto _label Break))))))
    (:0
      (Components|Activation|Deactivate (Variables|Default|GetChainBeam1)))
    (:1
      (Components|Activation|Deactivate (Variables|Default|GetChainBeam2))
      (goto _label))))

(fn CheckNearbyandUpdateBeams
  (bind (_outactors _returnvalue) (Class|KismetSystemLibrary|SphereOverlapActorsNEW (Transformation|GetActorLocation) (Variables|Default|GetGangOverlapRange) (Utilities|Array|MakeArray "ObjectTypeQuery7") "/Game/PrimalEarth/Dinos/Eel/Eel_Character_BP.Eel_Character_BP_C" (Utilities|Array|MakeArray self)))
  (if _returnvalue
    (CallFunction|UpdateChainBeamEnds _outactors)))

(fn BlueprintCanAttack
  (params (AttackIndex :type Integer) (distance :type Float%20%28single-precision%29) (attackRangeOffset :type Float%20%28single-precision%29) (OtherTarget :type Actor%20Object%20Reference))
  (LocalVariables|SetRetVal true)
  (switch int AttackIndex
    (:Default
      (return (LocalVariables|GetRetVal)))
    (:0
      (return (LocalVariables|GetRetVal)))
    (:1
      (return (LocalVariables|GetRetVal)))
    (:2
      (return (LocalVariables|GetRetVal)))
    (:3
      (bind _asprimalcharacter (Utilities|Casting|CastToPrimalCharacter OtherTarget)
        (:then
          (Utilities|FlowControl|Sequence
            (:then_0
              (bind _returnvalue (Class|PrimalCharacter|GetDragWeight _asprimalcharacter))
              (if (< (+ (Variables|Default|GetBaseShockWeight) (* (Variables|Default|GetGangCount) (Variables|Default|GetShockWeightPerGangBonus))) _returnvalue)
                (LocalVariables|SetRetVal false)))
            (:then_1
              (if (Variables|/Script/ShooterGame.PrimalCharacter|GetbPreventAllBuffs _asprimalcharacter)
                (LocalVariables|SetRetVal false)))
            (:then_2
              (return (LocalVariables|GetRetVal)))))
        (:CastFailed
          (return (LocalVariables|GetRetVal)))))))

(fn OnRepCanLightningAttack
  (bind _canlightningattackeffect (Variables|Default|GetCanLightningAttackEffect))
  (if (not (Networking|IsDedicatedServer))
    (if (Variables|Default|GetCanLightningAttack)
      (Components|Activation|Activate _canlightningattackeffect false)
      (CallFunction|UpdateEmissive)
      (else
        (Components|Activation|Deactivate _canlightningattackeffect)
        (CallFunction|UpdateEmissive)))))

(fn UpdateEmissive
  (bind _mesh (Variables|Character|GetMesh))
  (bind _returnvalue (Rendering|Material|GetMaterial _mesh 0))
  (if (Variables|Default|GetCanLightningAttack)
    (bind _asmaterialinstancedynamic (Utilities|Casting|CastToMaterialInstanceDynamic _returnvalue))
    (bind _returnvalue_2 (Rendering|Material|GetVectorParameterValue _asmaterialinstancedynamic "Emissive - Color and Intensity" :!class /Script/Engine.MaterialInstanceDynamic))
    (Rendering|Material|SetVectorParameterValue _asmaterialinstancedynamic "Emissive - Color and Intensity" (Utilities|Struct|MakeLinearColor (.R (Utilities|Struct|BreakLinearColor _returnvalue_2)) (.G (Utilities|Struct|BreakLinearColor _returnvalue_2)) (.B (Utilities|Struct|BreakLinearColor _returnvalue_2)) (Variables|Default|GetmaxEmissive)) :!class /Script/Engine.MaterialInstanceDynamic)
    (else
      (bind _asmaterialinstancedynamic_2 (Utilities|Casting|CastToMaterialInstanceDynamic _returnvalue))
      (bind _returnvalue_3 (Rendering|Material|GetVectorParameterValue _asmaterialinstancedynamic_2 "Emissive - Color and Intensity" :!class /Script/Engine.MaterialInstanceDynamic))
      (Rendering|Material|SetVectorParameterValue _asmaterialinstancedynamic_2 "Emissive - Color and Intensity" (Utilities|Struct|MakeLinearColor (.R (Utilities|Struct|BreakLinearColor _returnvalue_3)) (.G (Utilities|Struct|BreakLinearColor _returnvalue_3)) (.B (Utilities|Struct|BreakLinearColor _returnvalue_3)) (Variables|Default|GetminEmissive)) :!class /Script/Engine.MaterialInstanceDynamic))))

(fn BPSetupTamed
  (params (bWasJustTamed :type Boolean)))

(fn BPUnstasis
  (|CallParentFunction)
  (Variables|Default|SetCanLightningAttack true false))