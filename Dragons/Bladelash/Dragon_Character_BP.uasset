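; Dragon character Blueprint that announces to the server when the dragon gets tamed.
; Each tick on the server, it watches for its targeting team reaching the player-team range and latches a WasTamed flag so it fires once.
; It then casts the game mode to ShooterGameMode and sends a pink billboard notification with a dragon-head icon.
; The construction script only calls the parent.
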(event EventTick
  (params (DeltaSeconds :type Float%20%28single-precision%29))
  (|CallParentFunction DeltaSeconds)
  (if (Math|Boolean|ANDBoolean (Networking|IsServer) (not (Variables|Default|GetbWasTamed)) (>= (Variables|Default|GetTargetingTeam) 50000))
    (Variables|Default|SetbWasTamed true)
    (bind _asshootergamemode (Utilities|Casting|CastToShooterGameMode (Game|GetGameMode)))
    (Class|ShooterGameMode|SendServerNotification _asshootergamemode (Utilities|String|Append (Utilities|String|Append "THE DRAGON HAS BEEN TAMED!" "") "!") "(R=1.000000,G=0.054220,B=0.579979,A=1.000000)" 2.0 6.75 "/Game/PrimalEarth/UI/Empty_DragonHead_Icon.Empty_DragonHead_Icon" 0 -1 -1 true)))

(fn ConstructionScript
  (|CallParentFunction))