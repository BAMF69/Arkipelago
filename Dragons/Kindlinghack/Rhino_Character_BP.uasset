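; Rhino character Blueprint for a rideable creature whose built-up extra running speed boosts its melee damage, giving it a charge attack.
; GetExtraRunSpeedModifierPercent normalizes the best speed modifier between its min and max when the Rider check passes.
; That percent drives the HUD buff progress bar and scales the bonus melee damage.
; GetBestExtraRunSpeedModifier briefly holds the last higher speed value, so the bonus survives a momentary slowdown.
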(fn ConstructionScript
  (|CallParentFunction))

(fn GetExtraRunSpeedModifierPercent
  (bind _scaleextrarunningspeedmodifiermin (Variables|Default|GetScaleExtraRunningSpeedModifierMin))
  (if (== (Variables|Default|GetRider) 0)
    _
    (else
      (LocalVariables|SetPercentOut (/ (- (CallFunction|GetBestExtraRunSpeedModifier) _scaleextrarunningspeedmodifiermin) (- (Variables|Default|GetScaleExtraRunningSpeedModifierMax) _scaleextrarunningspeedmodifiermin)))))
  (return (LocalVariables|GetPercentOut)))

(fn BPGetHUDOverrideBuffProgressBarPercent
  (bind _percentval (CallFunction|GetExtraRunSpeedModifierPercent))
  (return _percentval))

(fn BPGetExtraMeleeDamageModifier
  (bind _percentval (CallFunction|GetExtraRunSpeedModifierPercent))
  (return (+ 1.0 (* (Variables|Default|GetMaxExtraSpeedAdditionalDamagePercent) _percentval))))

(fn GetBestExtraRunSpeedModifier
  (if (< (Math|Conversions|ToFloat(Integer) (- (Utilities|Time|GetGameTimeinSeconds) (Variables|Default|GetLastHigherScaleExtraRunningSpeedTime))) 0.55)
    (LocalVariables|SetretVal (Variables|Default|GetLastHigherScaleExtraRunningSpeedValue))
    (else
      (LocalVariables|SetretVal (Variables|Default|GetExtraRunningSpeedModifier))))
  (return (LocalVariables|GetretVal)))