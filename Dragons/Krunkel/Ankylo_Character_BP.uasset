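; Ankylo dino character Blueprint that restricts harvest damage by attack type and gates attacks by movement mode.
; Harvest damage passes only for attack 1 on Use harvest components or attacks 0 and 2 on Attack ones, otherwise zero.
; AI and rider checks allow only attack 0, while walking or swimming.
; In other movement modes, the rider check rejects attack 0 but fires attack 2 as a side effect if available.
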(fn ConstructionScript
  (|CallParentFunction))

(fn BPModifyHarvestDamage
  (params (harvestComponent :type Primal%20Harvesting%20Component%20Object%20Reference) (inDamage :type Float%20%28single-precision%29))
  (bind _currentattackindex (Variables|Default|GetCurrentAttackIndex))
  (return (Math|Float|SelectFloat inDamage 0.0 (or (and (Utilities|ClassIsChildOf (Utilities|GetClass harvestComponent) "/Game/PrimalEarth/CoreBlueprints/HarvestComponents/UseHarvestComponent_Base.UseHarvestComponent_Base_C") (== _currentattackindex 1)) (and (or (== _currentattackindex 0) (== _currentattackindex 2)) (Utilities|ClassIsChildOf (Utilities|GetClass harvestComponent) "/Game/PrimalEarth/CoreBlueprints/HarvestComponents/AttackHarvestComponent_Base.AttackHarvestComponent_Base_C"))))))

(fn BlueprintCanRiderAttack
  (params (AttackIndex :type Integer))
  (bind _charactermovement (Variables|Character|GetCharacterMovement))
  (bind _movementmode (Variables|/Script/Engine.CharacterMovementComponent|GetMovementMode _charactermovement))
  (LocalVariables|SetcanDoAttack false)
  (Utilities|FlowControl|Sequence
    (:then_0
      (if (== AttackIndex 0)
        (if (Utilities|IsValid _charactermovement)
          (if (or (Utilities|Enum|Equal(Enum) _movementmode "MOVE_Swimming") (Utilities|Enum|Equal(Enum) _movementmode "MOVE_Walking"))
            (bind _returnvalue (Class|PrimalDinoCharacter|CanAttack))
            (LocalVariables|SetcanDoAttack _returnvalue)
            (else
              (bind _returnvalue_2 (Class|PrimalDinoCharacter|CanAttack 2))
              (if _returnvalue_2
                (Class|PrimalDinoCharacter|DoAttack 2 true false)))))))
    (:then_1
      (return (LocalVariables|GetcanDoAttack)))))

(fn BlueprintCanAttack
  (params (AttackIndex :type Integer) (distance :type Float%20%28single-precision%29) (attackRangeOffset :type Float%20%28single-precision%29) (OtherTarget :type Actor%20Object%20Reference))
  (bind _charactermovement (Variables|Character|GetCharacterMovement))
  (bind _movementmode (Variables|/Script/Engine.CharacterMovementComponent|GetMovementMode _charactermovement))
  (LocalVariables|SetcanAttack false)
  (Utilities|FlowControl|Sequence
    (:then_0
      (if (== AttackIndex 0)
        (if (Utilities|IsValid _charactermovement)
          (if (or (Utilities|Enum|Equal(Enum) _movementmode "MOVE_Walking") (Utilities|Enum|Equal(Enum) _movementmode "MOVE_Swimming"))
            (bind _returnvalue (Class|PrimalDinoCharacter|CanAttack))
            (LocalVariables|SetcanAttack _returnvalue)))))
    (:then_1
      (return (LocalVariables|GetcanAttack)))))