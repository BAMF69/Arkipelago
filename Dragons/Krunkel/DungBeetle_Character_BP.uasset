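; Dung Beetle dino character that drives the timed crafting in its DinoTamedInventoryComponent_Beetle according to whether tamed wandering is enabled.
; Multi-use index 158 starts the crafting timers when wandering is on, otherwise attempts a final craft and clears them.
; On the server, waking restarts timers if wandering.
; Sleep and death clear them on the server, first attempting a craft if wandering.
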(event Custom|OnDied_Event
  (params (DiedCharacter :type Primal%20Character%20Object%20Reference))
  (if (Networking|IsServer)
    (bind _asdinotamedinventorycomponent_beetle_c (Utilities|Casting|CastToDinoTamedInventoryComponent_Beetle (Variables|Default|GetMyInventoryComponent)))
    (if (Variables|Default|GetbEnableTamedWandering)
      (Default|TrytoCraft _asdinotamedinventorycomponent_beetle_c)
      (Default|UnsetAll _asdinotamedinventorycomponent_beetle_c)
      (else
        (Default|UnsetAll _asdinotamedinventorycomponent_beetle_c)))))

(event EventBeginPlay
  (EventDispatchers|BindEventtoOnDied (delegate Custom|OnDied_Event)))

(fn ConstructionScript
  (|CallParentFunction))

(fn BPTryMultiUse
  (params (ForPC :type Player%20Controller%20Object%20Reference) (UseIndex :type Integer))
  (Utilities|FlowControl|Sequence
    (:then_0
      (if (== UseIndex 158)
        (bind _asdinotamedinventorycomponent_beetle_c (Utilities|Casting|CastToDinoTamedInventoryComponent_Beetle (Variables|Default|GetMyInventoryComponent)))
        (if (Variables|Default|GetbEnableTamedWandering)
          (Default|InitialSetCraftingTimes _asdinotamedinventorycomponent_beetle_c)
          (else
            (Default|TrytoCraft _asdinotamedinventorycomponent_beetle_c)
            (Default|UnsetAll _asdinotamedinventorycomponent_beetle_c)))))
    (:then_1
      (return true))))

(fn BPGetMultiUseEntries
  (params (ForPC :type Player%20Controller%20Object%20Reference) (MultiUseEntries :type Array%20of%20Multi%20Use%20Entry%20Structures))
  (return MultiUseEntries))

(fn BPCharacterUnsleeped
  (if (Networking|IsServer)
    (bind _asdinotamedinventorycomponent_beetle_c (Utilities|Casting|CastToDinoTamedInventoryComponent_Beetle (Variables|Default|GetMyInventoryComponent)))
    (if (Variables|Default|GetbEnableTamedWandering)
      (Default|InitialSetCraftingTimes _asdinotamedinventorycomponent_beetle_c))))

(fn BPCharacterSleeped
  (if (Networking|IsServer)
    (bind _asdinotamedinventorycomponent_beetle_c (Utilities|Casting|CastToDinoTamedInventoryComponent_Beetle (Variables|Default|GetMyInventoryComponent)))
    (if (Variables|Default|GetbEnableTamedWandering)
      (Default|TrytoCraft _asdinotamedinventorycomponent_beetle_c)
      (Default|UnsetAll _asdinotamedinventorycomponent_beetle_c)
      (else
        (Default|UnsetAll _asdinotamedinventorycomponent_beetle_c)))))