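; Dilo dinosaur character Blueprint that overrides the attack check to restrict which targets its attack index 1 may be used on.
; Other attack indices, tamed Dilos and those with a gameplay-relevant mesh are always allowed.
; Otherwise the attack is allowed only against ShooterCharacter targets or tamed dinos.
; The construction script only calls its parent.
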(fn ConstructionScript
  (|CallParentFunction))

(fn BlueprintCanAttack
  (params (AttackIndex :type Integer) (distance :type Float%20%28single-precision%29) (attackRangeOffset :type Float%20%28single-precision%29) (OtherTarget :type Actor%20Object%20Reference))
  (LocalVariables|SetCanAttack true)
  (if (Math|Boolean|ORBoolean (!= AttackIndex 1) (Class|PrimalDinoCharacter|BPIsTamed) (Class|PrimalCharacter|IsMeshGameplayRelevant))
    (return (LocalVariables|GetCanAttack))
    (else
      (Utilities|Casting|CastToShooterCharacter OtherTarget
        (:CastFailed
          (bind _asprimaldinocharacter (Utilities|Casting|CastToPrimalDinoCharacter OtherTarget)
            (:then
              (if (not (Class|PrimalDinoCharacter|BPIsTamed _asprimaldinocharacter))
                (LocalVariables|SetCanAttack false)))
            (:CastFailed
              (LocalVariables|SetCanAttack false))))))))