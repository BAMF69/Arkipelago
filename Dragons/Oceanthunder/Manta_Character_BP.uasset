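; Character Blueprint for the rideable Manta, an aquatic creature, driving its water-bound movement, land damage and surface effects from Tick.
; A rider lets it leave water and optionally locks pitch level; riderless, it is kept in water and flagged to die if it leaves.
; The server applies periodic max-health-scaled damage while it is walking with a rider.
; Non-dedicated instances spawn a splash on falling into water and toggle a trail while swimming near the surface.
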(event EventTick
  (params (DeltaSeconds :type Float%20%28single-precision%29))
  (bind _returnvalue (Utilities|Time|GetGameTimeinSeconds))
  (bind _returnvalue_2 (Transformation|GetActorRotation))
  (bind _returnvalue_3 (Networking|IsServer))
  (bind _returnvalue_4 (Class|PrimalCharacter|IsAlive))
  (bind _watertrailparticle (Variables|Default|GetWaterTrailParticle))
  (bind _charactermovement (Variables|Character|GetCharacterMovement))
  (bind (_pitch _yaw _roll) (Class|KismetMathLibrary|BreakRot _returnvalue_2))
  (bind _movementmode (Variables|/Script/Engine.CharacterMovementComponent|GetMovementMode _charactermovement))
  (bind _returnvalue_5 (Utilities|Enum|Equal(Enum) _movementmode "MOVE_Swimming"))
  (Utilities|FlowControl|Sequence
    (:then_0
      (if (!= (Variables|Default|GetRider) 0)
        (Variables|/Script/Engine.CharacterMovementComponent|SetbPreventExitingWater _charactermovement false)
        (Variables|Default|SetbDieIfLeftWater false)
        (Variables|Default|SetbFlyerForceNoPitch (Variables|Default|GetZeroRiderPitch))
        (if _returnvalue_3
          (Utilities|FlowControl|Sequence
            (:then_0
              (if (Variables|Default|GetZeroRiderPitch)
                (if (!= _pitch 0.0)
                  (Transformation|SetActorRotation (Math|Rotator|MakeRotator 0.0 _yaw _roll)))))
            (:then_1
              (if (and _returnvalue_4 (Utilities|Enum|Equal(Enum) _movementmode "MOVE_Walking")) :!label _label
                (if (and (> (Math|Conversions|ToFloat(Integer) (- _returnvalue (Variables|Default|GetLastLandDamageTime))) (Variables|Default|GetLandDamageTimeInterval)) (!= (Variables|Default|GetRider) 0))
                  (Variables|Default|SetLastLandDamageTime _returnvalue)
                  (Game|Damage|ApplyDamage self (* (Variables|Default|GetLandDamageTimeAmount) (Class|PrimalCharacter|GetMaxHealth)) 0 0 (Variables|Default|GetLandDamageType)))))))
        (else
          (Variables|/Script/Engine.CharacterMovementComponent|SetbPreventExitingWater _charactermovement true)
          (Variables|Default|SetbDieIfLeftWater true)
          (Variables|Default|SetbFlyerForceNoPitch false)
          (if _returnvalue_3
            (goto _label)))))
    (:then_1
      (if (not (Networking|IsDedicatedServer))
        (if _returnvalue_4
          (Utilities|FlowControl|Sequence
            (:then_0
              (if (and (Utilities|Enum|Equal(Enum) (Variables|Default|GetLastMovementMode) "MOVE_Falling") _returnvalue_5)
                (Game|SpawnActorfromClass (Variables|Default|GetSplashEmitter) (Transformation|GetActorTransform) true)))
            (:then_1
              (Variables|Default|SetLastMovementMode _movementmode))
            (:then_2
              (if (Math|Boolean|NotEqual(Boolean) (Variables|Default|GetbParticlesActivated) (Variables|Default|GetbIsTrailEffectActive))
                (Variables|Default|SetbParticlesActivated (Variables|Default|GetbIsTrailEffectActive))
                (if (Variables|Default|GetbParticlesActivated)
                  (Components|Activation|Activate _watertrailparticle true)
                  (else
                    (Components|Activation|Deactivate _watertrailparticle)))))))))
    (:then_2
      (if (!= (Pawn|GetController) 0)
        (if (and (< (Math|Conversions|ToFloat(Integer) (- (Utilities|Time|GetGameTimeinSeconds) (Variables|/Script/Engine.CharacterMovementComponent|GetPreventWaterHopping_LastTimeAtSurface _charactermovement))) 0.3) _returnvalue_5)
          (if (not (Variables|Default|GetbIsTrailEffectActive))
            (Variables|Default|SetbIsTrailEffectActive true false))
          (elif (Variables|Default|GetbIsTrailEffectActive)
            (Variables|Default|SetbIsTrailEffectActive false false)))))))

(fn ConstructionScript
  (|CallParentFunction))