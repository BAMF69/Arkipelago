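; Character Blueprint for the Pela, a rideable creature that flies and swims and allows its rider to use a fishing rod while swimming.
; On non-dedicated instances, Tick spawns splashes when it falls into water or takes flight from it, and toggles a water trail during fast swimming.
; For the local rider, the third-person camera eases to an offset view while fishing, and resets to class defaults on dismount.
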(event EventTick
  (params (DeltaSeconds :type Float%20%28single-precision%29))
  (bind _returnvalue (Transformation|GetActorTransform))
  (bind _default (CallFunction|GetDefaultPela))
  (bind _watertrailparticle (Variables|Default|GetWaterTrailParticle))
  (bind _rider (Variables|Default|GetRider))
  (bind _charactermovement (Variables|Character|GetCharacterMovement))
  (bind (_location _rotation) (Math|Transform|BreakTransform _returnvalue))
  (bind _velocity (Variables|/Script/Engine.MovementComponent|GetVelocity _charactermovement))
  (bind _tpvcameraoffset (Variables|/Script/ShooterGame.PrimalCharacter|GetTPVCameraOffset _default))
  (bind _movementmode (Variables|/Script/Engine.CharacterMovementComponent|GetMovementMode _charactermovement))
  (bind _returnvalue_2 (Math|Vector|VectorLength _velocity))
  (bind _returnvalue_3 (Utilities|Enum|Equal(Enum) _movementmode "MOVE_Swimming"))
  (bind _returnvalue_4 (> _returnvalue_2 2e+02))
  (bind _returnvalue_5 (and _returnvalue_4 _returnvalue_3))
  (if (not (Networking|IsDedicatedServer))
    (if (Class|PrimalCharacter|IsAlive)
      (Utilities|FlowControl|Sequence
        (:then_0
          (if (or (and (Utilities|Enum|Equal(Enum) (Variables|Default|GetLastMovementMode) "MOVE_Falling") _returnvalue_3) (and (Utilities|Enum|Equal(Enum) (Variables|Default|GetLastMovementMode) "MOVE_Swimming") (Utilities|Enum|Equal(Enum) _movementmode "MOVE_Flying")))
            (Game|SpawnActorfromClass (Variables|Default|GetSplashEmitter) (Math|Transform|MakeTransform (+ _location "0, 0,-90.000000") _rotation) true)))
        (:then_1
          (Variables|Default|SetLastMovementMode _movementmode))
        (:then_2
          (if (Math|Boolean|NotEqual(Boolean) (Variables|Default|GetbParticlesActivated) _returnvalue_5)
            (Variables|Default|SetbParticlesActivated _returnvalue_5)
            (if (Variables|Default|GetbParticlesActivated)
              (Components|Activation|Activate _watertrailparticle true)
              (else
                (Components|Activation|Deactivate _watertrailparticle)))))
        (:then_3
          (if (Pawn|IsLocallyControlled)
            (if (Variables|Default|GetbHasRider)
              (Utilities|IsValid _rider
                (:Is%20Valid
                  (if (Class|Actor|BPIsA (Variables|/Script/ShooterGame.ShooterCharacter|GetCurrentWeapon _rider) "/Game/PrimalEarth/CoreBlueprints/Weapons/WeapFishingRod.WeapFishingRod_C")
                    (CallFunction|InterpCameraTPV (+ (Variables|Default|GetFishingTPVCameraOffset) _tpvcameraoffset) DeltaSeconds)
                    (else
                      (CallFunction|InterpCameraTPV _tpvcameraoffset DeltaSeconds))))))))))))

(fn ConstructionScript
  (|CallParentFunction))

(fn InterpCameraTPV
  (params (targetOffset :type Vector) (deltaTime :type Float%20%28single-precision%29))
  (if (!= (Variables|Default|GetTPVCameraOffset) targetOffset)
    (if (Utilities|AreVectorsNearlyEqual (Variables|Default|GetTPVCameraOffset) targetOffset 0.5)
      (Variables|Default|SetTPVCameraOffset targetOffset)
      (else
        (Variables|Default|SetTPVCameraOffset (Math|Interpolation|VInterpTo (Variables|Default|GetTPVCameraOffset) targetOffset deltaTime (Variables|Default|GetInterpCameraSpeed)))))))

(fn BPNotifyClearRider
  (params (RiderClearing :type Shooter%20Character%20Object%20Reference))
  (|CallParentFunction RiderClearing)
  (Variables|Default|SetTPVCameraOffset (Variables|/Script/ShooterGame.PrimalCharacter|GetTPVCameraOffset (CallFunction|GetDefaultPela))))

(fn GetDefaultPela
  (bind _returnvalue (Class|VictoryCore|GetDefaultObject self))
  (bind _aspela_character_bp_c (Utilities|Casting|CastToPela_Character_BP _returnvalue))
  (return _aspela_character_bp_c))

(fn BPForceAllowMountedWeapon
  (params (WeaponTemplate :type Shooter%20Weapon%20Class%20Reference))
  (return (and (Utilities|Enum|Equal(Enum) (Variables|/Script/Engine.CharacterMovementComponent|GetMovementMode (Variables|Character|GetCharacterMovement)) "MOVE_Swimming") (Utilities|ClassIsChildOf WeaponTemplate "/Game/PrimalEarth/CoreBlueprints/Weapons/WeapFishingRod.WeapFishingRod_C"))))