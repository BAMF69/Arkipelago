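; DodoWyvern event boss character, with fire-breath particles spawned on anim notify and a flying offset passed to its anim Blueprint.
; After a server-side delay, a "Boss"-tagged instance notifies ModCommunication_Interface actors of its spawn, or destroys itself if none exist.
; Death broadcasts a slain notification, then unclaims same-team zombie wyverns and retags them "FearEvolved".
; Event tags are exchanged as JSON through mod-data messages.
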(event Custom|OnDied_Event
  (params (DiedCharacter :type Primal%20Character%20Object%20Reference))
  (bind _asshootergamemode (Utilities|Casting|CastToShooterGameMode (Game|GetGameMode)))
  (Class|ShooterGameMode|SendServerNotification _asshootergamemode "THE DODOWYVERN HAS BEEN SLAIN!" "(R=1.000000,G=0.520307,B=0.000000,A=1.000000)" 1.5 4.0 0 "/Game/PrimalEarth/Sound/SFX/Temp/ARK_Dodorex_Stinger.ARK_Dodorex_Stinger" -1 -1 false)
  (CallFunction|UnclaimMinions))

(event Custom|AnimNotify_BreatheFireEffect
  (for _array_element (Actor|GetComponentsByClass "/Script/Engine.SkeletalMeshComponent")
    (bind _asskeletalmeshcomponent (Utilities|Casting|CastToSkeletalMeshComponent _array_element))
    (if (and (Variables|/Script/Engine.SceneComponent|GetbVisible _asskeletalmeshcomponent) (not (Networking|IsDedicatedServer)))
      (Effects|SpawnEmitterAttached "/Game/ScorchedEarth/Effects/ParticleSystems/Creatures/Wyvern/P_Wyvern_Fire_Muzzle.P_Wyvern_Fire_Muzzle" _asskeletalmeshcomponent "FlameBreath_FX" "0, 0, 0" "0, 0, 0" "SnapToTarget")
      (Effects|SpawnEmitterAttached "/Game/PrimalEarth/Effects/Particles/Creatures/Dragon/P_Wyvern_Ground_FlameBreath.P_Wyvern_Ground_FlameBreath" _asskeletalmeshcomponent "FlameBreath_FX" "0, 0, 0" "0, 0, 0" "SnapToTarget"))))

(event EventSendModData
  (params (Key :type Name :default "None") (JsonData :type Json%20Object%20Object%20Reference))
  (Utilities|IsValid JsonData
    (:Is%20Valid
      (switch name Key
        (:SetEventTags
          (bind (_outvalue _returnvalue) (Class|JsonObject|GetStringArrayField JsonData "EventTags"))
          (if _returnvalue
            (Variables|Default|SetEventTags _outvalue)))))))

(event EventBeginPlay
  (bind _aswyvernanimblueprint_c (Utilities|Casting|CastToWyvernAnimBlueprint (Components|SkeletalMesh|GetAnimInstance (Variables|Character|GetMesh))))
  (Variables|/Game/PrimalEarth/CoreBlueprints/BaseAnimBlueprints/DinoBlueprintBase_RootTransformIK_FullFlight.DinoBlueprintBase_RootTransformIK_FullFlight_C|SetFlyingOffset _aswyvernanimblueprint_c (Variables|Default|GetNewFlyingOffset))
  (Networking|SwitchHasAuthority
    (:Authority
      (EventDispatchers|BindEventtoOnDied (delegate Custom|OnDied_Event))
      (Utilities|FlowControl|RetriggerableDelay 2.0)
      (if (Utilities|Array|ContainsItem (Variables|Default|GetEventTags) "Boss")
        (bind _outactors (Actor|GetAllActorswithInterface "/Game/PrimalEarth/CoreBlueprints/ModCommunication_Interface.ModCommunication_Interface_C"))
        (if (> (Utilities|Array|Length _outactors) 0)
          (Class|ModCommunicationInterface|SendModData(Message) _outactors "EventCreatureSpawned")
          (else
            (Actor|DestroyActor)))))))

(fn ConstructionScript
  (|CallParentFunction))

(fn UnclaimMinions
  (Networking|SwitchHasAuthority
    (:Authority
      (bind _returnvalue (Class|JsonObject|CreateJsonObject))
      (LocalVariables|SetJSONUnclaim _returnvalue)
      (Class|JsonObject|SetStringArrayField (LocalVariables|GetJSONUnclaim) "EventTags" (Utilities|Array|MakeArray "FearEvolved"))
      (bind _outactors (Actor|GetAllActorsOfClass "/Game/ScorchedEarth/Dinos/Wyvern/Wyvern_Character_BP_ZombieBase.Wyvern_Character_BP_ZombieBase_C"))
      (for _array_element _outactors
        (if (== (Variables|/Script/Engine.Actor|GetTargetingTeam _array_element) (Variables|Default|GetTargetingTeam))
          (bind _asprimaldinocharacter (Utilities|Casting|CastToPrimalDinoCharacter _array_element))
          (Class|PrimalDinoCharacter|UnclaimDino _asprimaldinocharacter true)
          (Class|ModCommunicationInterface|SendModData(Message) _asprimaldinocharacter "SetEventTags" (LocalVariables|GetJSONUnclaim)))))))

(fn RequestModData
  (params (Key :type Name :default "None"))
  (switch name Key
    (:GetEventTags
      (bind _returnvalue (Class|JsonObject|CreateJsonObject))
      (LocalVariables|SetJSONObject _returnvalue)
      (Class|JsonObject|SetStringArrayField (LocalVariables|GetJSONObject) "EventTags" (Variables|Default|GetEventTags))
      (return (LocalVariables|GetJSONObject)))))

(fn RequestModDataProcessing
  (params (Key :type Name :default "None") (InJsonData :type Json%20Object%20Object%20Reference))
  (return 0))