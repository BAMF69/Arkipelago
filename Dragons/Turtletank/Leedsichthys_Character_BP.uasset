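; Leedsichthys creature Blueprint: a giant fish that rams rafts, can be calmed with honey and scraped for meat.
; Its first attack on a PrimalRaft triggers a delayed, server-applied forward impulse.
; A server timer soothes it with underwater honey lures when it has a target and no recent character damage, eventually consuming the bait.
; A cooldown-gated multi-use grants weighted-random items; anim notifies spawn surface splashes at tail and mouth.
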(event Custom|ServerForceFwd
  (bind _returnvalue (Transformation|GetActorForwardVector))
  (bind (_x _y) (Math|Vector|BreakVector _returnvalue))
  (Class|PrimalCharacter|BPNetAddCharacterMovementImpulse (* (Math|Vector|Normalize (Math|Vector|MakeVector _x _y 0.01)) 3e+03) true 0.0 false "MOVE_None" false false))

(event Custom|Spawn%20Blood
  (params (ActorLocation :type Vector))
  (Effects|SpawnEmitteratLocation "/Game/PrimalEarth/Effects/Particles/Creatures/Leedsichthys/P_Leed_Harvest.P_Leed_Harvest" ActorLocation "0, 0, 0" true true 2e+03))

(event Custom|ForceFwd
  (bind _returnvalue (Transformation|GetActorForwardVector))
  (bind (_x _y) (Math|Vector|BreakVector _returnvalue))
  (Utilities|FlowControl|Delay 0.75)
  (if (Networking|IsServer)
    (Class|PrimalCharacter|BPNetAddCharacterMovementImpulse (* (Math|Vector|Normalize (Math|Vector|MakeVector _x _y 0.01)) 3e+03) true 0.0 false "MOVE_None" false false)
    (else
      (CallFunction|ServerForceFwd))))

(event Custom|AnimNotify_MouthSplash
  (bind _returnvalue (Pawn|GetMovementComponent))
  (bind _mesh (Variables|Character|GetMesh))
  (bind _returnvalue_2 (Transformation|GetSocketLocation _mesh "MouthSocket"))
  (bind _returnvalue_3 (Class|MovementComponent|GetPhysicsVolume _returnvalue))
  (bind (_origin _boxextent) (Collision|GetActorBounds _returnvalue_3 false))
  (bind (_x _y _z) (Math|Vector|BreakVector _returnvalue_2))
  (bind _z_2 (Math|Vector|BreakVector _origin))
  (bind _z_3 (Math|Vector|BreakVector _boxextent))
  (bind _returnvalue_4 (+ _z_2 _z_3))
  (if (not (Networking|IsDedicatedServer))
    (if (> _z _returnvalue_4)
      (Effects|SpawnEmitteratLocation "/Game/PrimalEarth/Effects/Particles/Creatures/Leedsichthys/P_Leed_WaterBreach.P_Leed_WaterBreach" (Math|Vector|MakeVector _x _y _returnvalue_4) "0, 0, 0" true true 2e+03))))

(event Custom|AnimNotify_TailSplash
  (bind _returnvalue (Pawn|GetMovementComponent))
  (bind _mesh (Variables|Character|GetMesh))
  (bind _returnvalue_2 (Transformation|GetSocketLocation _mesh "TailSocket"))
  (bind _returnvalue_3 (Class|MovementComponent|GetPhysicsVolume _returnvalue))
  (bind (_x _y _z) (Math|Vector|BreakVector _returnvalue_2))
  (bind (_origin _boxextent) (Collision|GetActorBounds _returnvalue_3 false))
  (bind _z_2 (Math|Vector|BreakVector _origin))
  (bind _z_3 (Math|Vector|BreakVector _boxextent))
  (bind _returnvalue_4 (+ _z_2 _z_3))
  (if (not (Networking|IsDedicatedServer))
    (if (> _z _returnvalue_4)
      (Effects|SpawnEmitteratLocation "/Game/PrimalEarth/Effects/Particles/Creatures/Leedsichthys/P_Leed_WaterBreach.P_Leed_WaterBreach" (Math|Vector|MakeVector _x _y _returnvalue_4) "0, 0, 0" true true 2e+03))))

(event Custom|SootheBehavior
  (bind _returnvalue (Transformation|GetActorLocation))
  (bind _self self)
  (bind _self_2 self)
  ;[1 0.7634 0] If honey is nearby, let it distract/soothe the leed
  (Utilities|IsValid (Variables|Default|GetTarget)
    (:Is%20Valid
      (if (Class|VictoryCore|IsTimeSince (Class|Actor|GetWorld) (Variables|Default|GetLastTimeTookDamage) 15.0 true)
        (bind _outhits (Collision|MultiSphereTraceForObjects _returnvalue (+ _returnvalue "0, 0,-1.000000") (Variables|Default|GetBaitCheckRadius) (Utilities|Array|MakeArray "ObjectTypeQuery11") false 0 "None"))
        (for _array_element _outhits
          (bind _asdroppeditemgeneric_honeylure_c (Utilities|Casting|CastToDroppedItemGeneric_HoneyLure (.HitActor (Collision|BreakHitResult _array_element))))
          (if (Variables|/Script/ShooterGame.DroppedItem|GetbIsUnderwater _asdroppeditemgeneric_honeylure_c)
            (Class|PrimalBuff|StaticAddBuff (Variables|Default|GetBaitSootheBuff) _self 0 _self false)
            (bind _asdino_aicontroller_bp_c (Utilities|Casting|CastToDino_AIController_BP (Pawn|GetController)))
            (Default|SetMovePointNearLure _asdroppeditemgeneric_honeylure_c _self_2 _asdino_aicontroller_bp_c)
            (bind _returnvalue_2 (Default|IsDinoinConsumeRange _asdroppeditemgeneric_honeylure_c _self_2 _asdino_aicontroller_bp_c))
            (if _returnvalue_2
              (Utilities|FlowControl|Sequence
                (:then_0
                  (Utilities|FlowControl|DoOnce false
                    (:Completed
                      (Variables|Default|SetBaitFoundTime (Utilities|Time|GetGameTimeinSeconds)))))
                (:then_1
                  (if (and (Class|VictoryCore|IsTimeSince (Class|Actor|GetWorld) (Variables|Default|GetBaitFoundTime) (Variables|Default|GetBaitDestroyAfterDuration) false) (!= (Math|Conversions|ToFloat(Integer) (Variables|Default|GetBaitFoundTime)) 0.0))
                    (Default|DestroyBait _asdroppeditemgeneric_honeylure_c)
                    (CallFunction|ClearBaitTime :!label _label)))
                (:then_2
                  (Utilities|FlowControl|RetriggerableDelay 1e+01)
                  (goto _label))))))))))

(event Custom|ClearBaitTime
  ;[1 0.2664 0.1515] Clear Bait Time
  (Variables|Default|SetBaitFoundTime 0.0)
  ;[1 0.7634 0] If honey is nearby, let it distract/soothe the leed
  (Utilities|FlowControl|DoOnce false) ; enters at Reset
)

(event EventBeginPlay
  (Variables|Default|SetTimeOfLastHarvest -1e+04 false)
  (Variables|Default|SetLastTimeTookDamage -1e+04))

(event EventBPTimerServer
  ;[0.06782 0.08 0.02934] Server Timer (for soothing)
  (CallFunction|SootheBehavior))

(fn ConstructionScript
  (|CallParentFunction))

(fn BPTryMultiUse
  (params (ForPC :type Player%20Controller%20Object%20Reference) (UseIndex :type Integer))
  (bind _returnvalue (Pawn|GetControlledPawn ForPC))
  (bind _harvestablenum (Variables|Harvesting|GetHarvestableNum))
  (bind _asprimalcharacter (Utilities|Casting|CastToPrimalCharacter _returnvalue)
    (:then
      (Utilities|FlowControl|Sequence
        (:then_0
          (switch int UseIndex
            (:977740
              (Variables|Default|SetTimeOfLastHarvest (Utilities|Time|GetGameTimeinSeconds) false)
              (bind _index (CallFunction|GetHarvestingIndex))
              (Utilities|FlowControl|Sequence
                (:then_0
                  (bind _returnvalue_2 (Class|VictoryCore|GetClassDefaultObject (Utilities|Array|Get(acopy) (Variables|Harvesting|GetHarvestableItems) _index)))
                  (bind _asprimalitem_base_c (Utilities|Casting|CastToPrimalItem_Base _returnvalue_2))
                  (bind (_numofstacks _leftover) (CallFunction|GetNumOfStackstoAdd (Variables|/Script/ShooterGame.PrimalItem|GetMaxItemQuantity _asprimalitem_base_c) (Math|Integer|SelectInt (Utilities|Array|Get(acopy) _harvestablenum _index) 1 (< _index (Utilities|Array|Length _harvestablenum)))))
                  (for _index_2 (range 1 _numofstacks)
                    (Class|PrimalItem|AddNewItem (Utilities|Array|Get(acopy) (Variables|Harvesting|GetHarvestableItems) _index) (Variables|/Script/ShooterGame.PrimalCharacter|GetMyInventoryComponent _asprimalcharacter) false false 0.0 false (Variables|/Script/ShooterGame.PrimalItem|GetMaxItemQuantity _asprimalitem_base_c) false 0.0 false 0 0.0))
                  (if (> _leftover 0)
                    (Class|PrimalItem|AddNewItem (Utilities|Array|Get(acopy) (Variables|Harvesting|GetHarvestableItems) _index) (Variables|/Script/ShooterGame.PrimalCharacter|GetMyInventoryComponent _asprimalcharacter) false false 0.0 false _leftover false 0.0 false 0 0.0)))
                (:then_1
                  (bind _asshootercharacter (Utilities|Casting|CastToShooterCharacter _returnvalue)
                    (:then
                      (bind _asanimmontage (Utilities|Casting|CastToAnimMontage (Utilities|SelectObject "/Game/PrimalEarth/Human/Female/Animations/Female-Pickup_Montage.Female-Pickup_Montage" "/Game/PrimalEarth/Human/Male/Animations/Human-Pickup_Montage.Human-Pickup_Montage" (Variables|/Script/ShooterGame.ShooterCharacter|GetbIsFemale _asshootercharacter)))
                        (:then
                          (Class|PrimalCharacter|PlayAnimEx _asprimalcharacter _asanimmontage 1.0 "None" true true false false false 0.0 0.0))
                        (:CastFailed
                          _)))
                    (:CastFailed
                      _))
                  (if (Class|PrimalCharacter|BPIsConscious)
                    (Class|PrimalCharacter|PlayAnimEx (Variables|Default|GetHarvestFishAnimMontage) 1.0 "None" true false false false false 0.0 0.0))
                  (Networking|ForceNetUpdate)
                  (CallFunction|SpawnBlood (+ (Transformation|GetActorLocation _asshootercharacter) (* (Math|Vector|GetForwardVector (Variables|/Script/Engine.Actor|GetStasisCheckComponent _asshootercharacter)) 1e+02))))))))
        (:then_1
          (return true))))
    (:CastFailed
      (return true))))

(fn BPGetMultiUseEntries
  (params (ForPC :type Player%20Controller%20Object%20Reference) (MultiUseEntries :type Array%20of%20Multi%20Use%20Entry%20Structures))
  (bind _harvestestingcooldown (Variables|Default|GetHarvestestingCooldown))
  (bind _asshootergamestate (Utilities|Casting|CastToShooterGameState (Game|GetGameState))
    (:then
      (bind _returnvalue (Class|ShooterGameState|GetNetworkTimeDelta _asshootergamestate (Variables|Default|GetTimeOfLastHarvest) false))
      (if (Class|Actor|IsDead)
        _
        (else
          (bind _returnvalue_2 (Class|VictoryCore|FormatasTime (Math|Float|Ceil (- _harvestestingcooldown (Math|Conversions|ToFloat(Integer) _returnvalue))) true false true))
          (Utilities|Array|Add MultiUseEntries (Utilities|Struct|MakeMultiUseEntry 0 (Utilities|String|ToString(Text) (Utilities|Text|FormatText "Scrape Meat {0}" (Utilities|Text|ToText(String) (Utilities|String|SelectString (Utilities|String|ToString(Text) (Utilities|Text|FormatText ": Wait Time {0}" (Utilities|Text|ToText(String) _returnvalue_2))) "" (not (>= (Math|Conversions|ToFloat(Integer) _returnvalue) _harvestestingcooldown)))))) 977740 1000 false (not (>= (Math|Conversions|ToFloat(Integer) _returnvalue) _harvestestingcooldown)) false false false false false false false true false false false false 0 (Math|Color|MakeColor 200 200 200 200) (Math|Conversions|ToColor(LinearColor) "(R=1.000000,G=0.696103,B=0.195000,A=1.000000)"))))))
    (:CastFailed
      _))
  (return MultiUseEntries))

(fn GetHarvestingIndex
  (LocalVariables|SetretIndex 0)
  (LocalVariables|SetSumOfWeights 0.0)
  (for _array_element (Variables|Harvesting|GetHarvestableWeights)
    (LocalVariables|SetSumOfWeights (+ _array_element (LocalVariables|GetSumOfWeights))))
  (LocalVariables|SetSelector (Math|Random|RandomFloatinRange 0.0 (LocalVariables|GetSumOfWeights)))
  (LocalVariables|SetWeightSumsAquiredSoFar 0.0)
  (bind (_array_element_2 _array_index) (Utilities|Array|ForEachLoopwithBreak (Variables|Harvesting|GetHarvestableWeights) :!label _label)
    (:LoopBody
      (LocalVariables|SetWeightSumsAquiredSoFar (+ _array_element_2 (LocalVariables|GetWeightSumsAquiredSoFar)))
      (if (<= (LocalVariables|GetSelector) (LocalVariables|GetWeightSumsAquiredSoFar))
        (LocalVariables|SetretIndex _array_index)
        (goto _label Break)))
    (:Completed
      (return (LocalVariables|GetretIndex)))))

(fn ReceiveAnyDamage
  (params (Damage :type Float%20%28single-precision%29) (DamageType :type Damage%20Type%20Object%20Reference) (InstigatedBy :type Controller%20Object%20Reference) (DamageCauser :type Actor%20Object%20Reference))
  (Utilities|Casting|CastToPrimalCharacter DamageCauser)
  (Variables|Default|SetLastTimeTookDamage (Utilities|Time|GetGameTimeinSeconds)))

(fn BPDoAttack
  (params (AttackIndex :type Integer))
  (switch int AttackIndex
    (:0
      (Utilities|Casting|CastToPrimalRaft (Variables|Default|GetTarget))
      (CallFunction|ForceFwd))))

(fn BPClientDoMultiUse
  (params (ForPC :type Player%20Controller%20Object%20Reference) (ClientUseIndex :type Integer))
  (switch int ClientUseIndex
    (:977740
      (bind _asshootercharacter (Utilities|Casting|CastToShooterCharacter (Pawn|GetControlledPawn ForPC)))
      (Class|ShooterWeapon|PlayWeaponAnimation (Variables|/Script/ShooterGame.ShooterCharacter|GetCurrentWeapon _asshootercharacter) (Utilities|Struct|MakeWeaponAnim "/Game/PrimalEarth/HumanMaleFPVHands/Animations/FPV_NoWeapon_Harvesting_Montage.FPV_NoWeapon_Harvesting_Montage") false false false false false false))))

(fn GetNumOfStackstoAdd
  (params (StackQuantity :type Integer) (NumToAdd :type Integer))
  (bind _returnvalue (/ NumToAdd StackQuantity))
  (return _returnvalue (- NumToAdd (* _returnvalue StackQuantity))))