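; Mosasaurus dino character Blueprint that relays rider input and events to its Tek helmet buff (Buff_DinoTekHelmet_Base).
; Each hook searches the creature's buffs for the helmet, so the weapon logic itself lives in the buff.
; Primary attack fires the helmet, secondary attack enables targeting with a narrowed FOV until targeting stops, and alt-fire or right thumbstick press triggers its alt fire.
; Clearing the rider deactivates an active helmet.
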(event Input|ActionEvents|InputActionGamepadRightThumbstick
  (:Pressed
    (bind _array_element (Utilities|Array|ForEachLoopwithBreak (Class|PrimalCharacter|GetBuffs) :!label _label)
      (:LoopBody
        (bind _asbuff_dinotekhelmet_base_c (Utilities|Casting|CastToBuff_DinoTekHelmet_Base _array_element))
        (Default|PressedAltFire _asbuff_dinotekhelmet_base_c)
        (goto _label Break)))))

(event Input|ActionEvents|InputActionAltFire
  (:Pressed
    (bind _array_element (Utilities|Array|ForEachLoopwithBreak (Class|PrimalCharacter|GetBuffs) :!label _label)
      (:LoopBody
        (bind _asbuff_dinotekhelmet_base_c (Utilities|Casting|CastToBuff_DinoTekHelmet_Base _array_element))
        (Default|PressedAltFire _asbuff_dinotekhelmet_base_c)
        (goto _label Break)))))

(fn ConstructionScript
  (|CallParentFunction))

(fn BPHandleonStopTargeting
  (bind _array_element (Utilities|Array|ForEachLoopwithBreak (Class|PrimalCharacter|GetBuffs) :!label _label)
    (:LoopBody
      (bind _asbuff_dinotekhelmet_base_c (Utilities|Casting|CastToBuff_DinoTekHelmet_Base _array_element))
      (Default|SetTargeting _asbuff_dinotekhelmet_base_c false)
      (goto _label Break))
    (:Completed
      (return false))))

(fn BPHandleControllerInitiatedAttack
  (params (AttackIndex :type Integer))
  (Utilities|FlowControl|Sequence
    (:then_0
      (bind _array_element (Utilities|Array|ForEachLoopwithBreak (Class|PrimalCharacter|GetBuffs) :!label _label)
        (:LoopBody
          (bind _asbuff_dinotekhelmet_base_c (Utilities|Casting|CastToBuff_DinoTekHelmet_Base _array_element))
          (if (== AttackIndex 0)
            (bind _bdidattack (Default|LocalDoAttack _asbuff_dinotekhelmet_base_c))
            (LocalVariables|SetretVal _bdidattack)
            (goto _label Break)
            (elif (== AttackIndex 1)
              (Default|SetTargeting _asbuff_dinotekhelmet_base_c true)
              (LocalVariables|SetretVal (Variables|/Game/PrimalEarth/CoreBlueprints/Buffs/Buff_DinoTekHelmet_Base.Buff_DinoTekHelmet_Base_C|GetbIsTargetingModeEnabled _asbuff_dinotekhelmet_base_c))
              (goto _label Break)
              (else
                (goto _label Break)))))))
    (:then_1
      (return (LocalVariables|GetretVal)))))

(fn BPNotifyClearRider
  (params (RiderClearing :type Shooter%20Character%20Object%20Reference))
  (bind _array_element (Utilities|Array|ForEachLoopwithBreak (Class|PrimalCharacter|GetBuffs))
    (:LoopBody
      (bind _asbuff_dinotekhelmet_base_c (Utilities|Casting|CastToBuff_DinoTekHelmet_Base _array_element))
      (if (Variables|/Game/PrimalEarth/CoreBlueprints/Buffs/Buff_DinoTekHelmet_Base.Buff_DinoTekHelmet_Base_C|GetbHelmetActivated _asbuff_dinotekhelmet_base_c)
        (Default|DeactivateHelmet _asbuff_dinotekhelmet_base_c)))))

(fn BPModifyFOV
  (params (FOVIn :type Float%20%28single-precision%29))
  (LocalVariables|SetretVal FOVIn)
  (Utilities|FlowControl|Sequence
    (:then_0
      (bind _array_element (Utilities|Array|ForEachLoopwithBreak (Class|PrimalCharacter|GetBuffs) :!label _label)
        (:LoopBody
          (bind _asbuff_dinotekhelmet_base_c (Utilities|Casting|CastToBuff_DinoTekHelmet_Base _array_element))
          (if (Variables|/Game/PrimalEarth/CoreBlueprints/Buffs/Buff_DinoTekHelmet_Base.Buff_DinoTekHelmet_Base_C|GetbIsTargetingModeEnabled _asbuff_dinotekhelmet_base_c)
            (LocalVariables|SetretVal 55.0)
            (goto _label Break)
            (else
              (goto _label Break))))))
    (:then_1
      (return (LocalVariables|GetretVal)))))